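; Actor component on the third-person character that handles item pickup and the equipment inventory screen.
; Interaction sphere-traces forward from the follow camera, adds a hit BP_Weapon's item data to the slot array and destroys the weapon actor.
; The inventory toggle creates or removes the WB_Equipment widget, switching cursor and input mode, freezing movement and blocking attacks via the attack system component while open.
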(event Custom|HandleItemInteract
  (bind _follow_camera (Variables|Default|GetFollow%20Camera))
  (bind _returnvalue (Transformation|GetWorldLocation _follow_camera))
  ;[1 1 1] Item Pick Up
  (bind (_outhit _returnvalue_2) (Collision|SphereTraceForObjects _returnvalue (+ _returnvalue (* (Math|Vector|GetForwardVector (Transformation|GetWorldRotation _follow_camera)) 1e+03)) 15.0 (Utilities|Array|MakeArray "ObjectTypeQuery2") false 0 "ForDuration"))
  (if _returnvalue_2
    (bind _asbp_weapon (Utilities|Casting|CastToBP_Weapon (.HitActor (Collision|BreakHitResult _outhit))))
    (CallFunction|AddItem (Variables|/Game/Equipment_system/BP_Weapon.BP_Weapon_C|GetItemData _asbp_weapon))
    (Actor|DestroyActor _asbp_weapon)
    (Development|PrintString "Item Picked up.")))

(event Custom|InventoryToggle
  (bind _returnvalue (Game|GetPlayerController 0))
  (bind _bpc_attack_system (Variables|Default|GetBPC%20Attack%20System))
  ;[1 1 1] Inventoy Toggle
  (if (not (Variables|Default|GetInventorOpened))
    (Variables|/Game/Blueprints/BPC_AttackSystem.BPC_AttackSystem_C|SetCanAttack _bpc_attack_system false)
    (bind _returnvalue_2 (UserInterface|CreateWidget "/Game/Equipment_system/UI/WB_Equipment.WB_Equipment_C"))
    (bind _output_get (Variables|Default|SetEquipmentWidget _returnvalue_2))
    (UserInterface|Viewport|AddtoViewport _output_get 0)
    (Variables|Default|SetInventorOpened true)
    (Variables|/Script/Engine.PlayerController|SetbShowMouseCursor _returnvalue true)
    (Input|SetInputModeGameandUI _returnvalue (Variables|Default|GetEquipmentWidget) "DoNotLock" true)
    (bind _asthird_person_character (Utilities|Casting|CastToThirdPersonCharacter (Components|GetOwner)))
    (Pawn|Components|CharacterMovement|SetMovementMode (Variables|/Script/Engine.Character|GetCharacterMovement _asthird_person_character) "MOVE_None" 0)
    (else
      (Variables|/Game/Blueprints/BPC_AttackSystem.BPC_AttackSystem_C|SetCanAttack _bpc_attack_system true)
      (bind _equipmentwidget (Variables|Default|GetEquipmentWidget)
        (:then
          (Widget|RemovefromParent _equipmentwidget)
          (Variables|Default|SetEquipmentWidget 0)
          (Variables|Default|SetInventorOpened false)
          (Variables|/Script/Engine.PlayerController|SetbShowMouseCursor _returnvalue false)
          (Input|SetInputModeGameOnly _returnvalue)
          (bind _asthird_person_character_2 (Utilities|Casting|CastToThirdPersonCharacter (Components|GetOwner)))
          (Pawn|Components|CharacterMovement|SetMovementMode (Variables|/Script/Engine.Character|GetCharacterMovement _asthird_person_character_2) "MOVE_Walking" 0))
        (:else)))))

(event EventBeginPlay
  (bind _asthird_person_character (Utilities|Casting|CastToThirdPersonCharacter (Components|GetOwner)))
  (Variables|Default|SetFollow%20Camera (Variables|/Game/ThirdPersonBP/Blueprints/ThirdPersonCharacter.ThirdPersonCharacter_C|GetFollowCamera _asthird_person_character))
  (Variables|Default|SetBPC%20Attack%20System (Variables|/Game/ThirdPersonBP/Blueprints/ThirdPersonCharacter.ThirdPersonCharacter_C|GetBPC_AttackSystem _asthird_person_character)))

(fn AddItem
  (params (NewItem :type S%20Slots%20Structure%20%28by%20ref%29))
  (Utilities|Array|Add (Variables|Default|GetItemSlots) NewItem))