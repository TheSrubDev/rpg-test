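; Quest component that tracks the active quest's elimination and chest objectives and shows them on a quest HUD widget created at BeginPlay.
; EliminateActor removes enemies from a working array copied from the objective, completing it when empty, while ChestOpened completes objectives matching that chest.
; Both update objective structs by reference and feed ObjectiveCompleted.
; Once all objectives finish, it grants experience through the player's stats component, clears the quest and plays completion animation and sound.
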(event Custom|SetText
  (Rendering|Components|TextRender|SetText (Variables|/Game/Quest_System/WB_QuestHUD.WB_QuestHUD_C|GetActiveQuest (Variables|Default|GetQuestHUDWidget)) (Utilities|Text|ToText(String) (.Name (Utilities|Struct|BreakS_Quests (Variables|Default|GetActiveQuest)))))
  (Default|ShowQuestPanel (Variables|Default|GetQuestHUDWidget)))

(event Custom|SetCurrentObjectives
  (Default|FillObjectives (Variables|Default|GetQuestHUDWidget) (.Objective (Utilities|Struct|BreakS_Quests (Variables|Default|GetActiveQuest)))))

(event Custom|EliminateActor
  (params (EnemyEliminated :type Actor%20Object%20Reference))
  (for _array_element (.objective (Variables|Default|GetActiveQuest))
    (if (and (not (.IsCompleted (Utilities|Struct|BreakS_QuestObjectives _array_element))) (.IsEliminateQuestObjective (Utilities|Struct|BreakS_QuestObjectives _array_element)))
      (if (!= (Utilities|Array|Length (Variables|Default|GetEnemyActorsArray)) 0)
        _
        (else
          (bind _output_get (Variables|Default|SetEnemyActorsArray (.ActorsToEliminate (Utilities|Struct|BreakS_QuestObjectives _array_element))))))
      (Utilities|Array|RemoveItem _output_get EnemyEliminated)
      (|SetBy-RefVar _array_element (Utilities|Struct|MakeS_QuestObjectives (.Objective (Utilities|Struct|BreakS_QuestObjectives _array_element)) false (Variables|Default|GetEnemyActorsArray) (.ChestToOpen (Utilities|Struct|BreakS_QuestObjectives _array_element)) (.IsEliminateQuestObjective (Utilities|Struct|BreakS_QuestObjectives _array_element)) (.IsChestObjective (Utilities|Struct|BreakS_QuestObjectives _array_element))))
      (Development|PrintString (Utilities|String|ToString(Integer) (Utilities|Array|Length (Variables|Default|GetEnemyActorsArray))))
      (if (== (Utilities|Array|Length (Variables|Default|GetEnemyActorsArray)) 0)
        (|SetBy-RefVar _array_element (Utilities|Struct|MakeS_QuestObjectives (.Objective (Utilities|Struct|BreakS_QuestObjectives _array_element)) true 0 (.ChestToOpen (Utilities|Struct|BreakS_QuestObjectives _array_element)) (.IsEliminateQuestObjective (Utilities|Struct|BreakS_QuestObjectives _array_element)) (.IsChestObjective (Utilities|Struct|BreakS_QuestObjectives _array_element))))
        (Default|CompleteObjective (Variables|Default|GetQuestHUDWidget) _array_element)
        (CallFunction|ObjectiveCompleted)
        (Development|PrintString "Elimination Objective Completed!")))))

(event Custom|ChestOpened
  (params (Chest :type Actor%20Object%20Reference))
  (for _array_element (.objective (Variables|Default|GetActiveQuest))
    (if (and (== Chest (.ChestToOpen (Utilities|Struct|BreakS_QuestObjectives _array_element))) (.IsChestObjective (Utilities|Struct|BreakS_QuestObjectives _array_element)))
      (|SetBy-RefVar _array_element (Utilities|Struct|MakeS_QuestObjectives (.Objective (Utilities|Struct|BreakS_QuestObjectives _array_element)) true (.ActorsToEliminate (Utilities|Struct|BreakS_QuestObjectives _array_element)) 0 (.IsEliminateQuestObjective (Utilities|Struct|BreakS_QuestObjectives _array_element)) (.IsChestObjective (Utilities|Struct|BreakS_QuestObjectives _array_element))))
      (Default|CompleteObjective (Variables|Default|GetQuestHUDWidget) _array_element)
      (CallFunction|ObjectiveCompleted)
      (Development|PrintString "Chest Objective Completed!"))))

(event Custom|ObjectiveCompleted
  (Math|Integer|IncrementInt (Variables|Default|GetObjectivesCompleted)
    (:%20%20
      (if (>= (Variables|Default|GetObjectivesCompleted) (Utilities|Array|Length (.objective (Variables|Default|GetActiveQuest))))
        (bind _asthird_person_character (Utilities|Casting|CastToThirdPersonCharacter (Game|GetPlayerCharacter 0)))
        (Default|IncreaseExperience (Variables|/Game/ThirdPersonBP/Blueprints/ThirdPersonCharacter.ThirdPersonCharacter_C|GetBPC_Player_Stats _asthird_person_character) (.reward_exp (Variables|Default|GetActiveQuest)))
        (Variables|Default|SetActiveQuest "")
        (Variables|Default|SetObjectivesCompleted 0)
        (Default|PlayQuestCompletedAnimation (Variables|Default|GetQuestHUDWidget))
        (Audio|PlaySound2D "/Game/Audio/UI/level_up_1.level_up_1" 1.0 1.0 0.0 0 0)))))

(event EventBeginPlay
  (bind _returnvalue (UserInterface|CreateWidget "/Game/Quest_System/WB_QuestHUD.WB_QuestHUD_C"))
  (bind _output_get (Variables|Default|SetQuestHUDWidget _returnvalue))
  (UserInterface|Viewport|AddtoViewport _output_get 0)
  (Default|HideQuestPanel (Variables|Default|GetQuestHUDWidget)))