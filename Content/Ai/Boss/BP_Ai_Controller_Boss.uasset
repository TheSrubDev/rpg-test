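; AI controller for a boss enemy that runs the boss behavior tree on BeginPlay and manages the boss fight's health bar and music.
; StartBossCombat adds the health bar widget to the viewport and spawns 2D music, and StopBossCombat removes the widget and stops the music.
; Tick sets the bar's percent from current over max health while the widget is valid.
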(event Custom|StartBossCombat
  (bind _returnvalue (UserInterface|CreateWidget "/Game/UI/WB_Boss_HealthBar.WB_Boss_HealthBar_C"))
  (bind _output_get (Variables|Default|SetBossHealthBarWidget _returnvalue))
  (UserInterface|Viewport|AddtoViewport _output_get 0)
  (bind _returnvalue_2 (Audio|SpawnSound2D "/Game/StarterContent/Audio/Starter_Music_Cue.Starter_Music_Cue" 1.0 1.0 0.0 0))
  (Variables|Default|SetBoss%20music _returnvalue_2))

(event Custom|StopBossCombat
  (Widget|RemovefromParent (Variables|Default|GetBossHealthBarWidget))
  (Variables|Default|SetBossHealthBarWidget 0)
  (Audio|Components|Audio|Stop (Variables|Default|GetBoss%20music)))

(event EventBeginPlay
  (AI|RunBehaviorTree "/Game/Ai/Boss/BT_Ai_Boss.BT_Ai_Boss"))

(event EventTick
  (params (DeltaSeconds :type Float%20%28single-precision%29))
  (bind _bosshealthbarwidget (Variables|Default|GetBossHealthBarWidget)
    (:then
      (Progress|SetPercent (Variables|/Game/UI/WB_Boss_HealthBar.WB_Boss_HealthBar_C|GetHealth_Bar _bosshealthbarwidget) (/ (Variables|Default|GetCurrentHealth) (Variables|Default|GetMaxHealth))))
    (:else)))

(fn ConstructionScript
  (|CallParentFunction))