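; Boss AI Blueprint that mirrors its health to its dedicated AI controller.
; Each Tick, after running the parent logic, it casts its controller to BP_Ai_Controller_Boss and copies current and max health from its BPCPlayerStats component.
; The controller is updated by per-frame polling, and the construction script only calls the parent.
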(event EventBeginPlay
  (|CallParentFunction) ; This node is disabled and will not be called.\nDrag off pins to build functionality.
)

(event Collision|EventActorBeginOverlap
  (params (OtherActor :type Actor%20Object%20Reference)))

(event EventTick
  (params (DeltaSeconds :type Float%20%28single-precision%29))
  (bind _bpc_player_stats (Variables|Default|GetBPC_Player_Stats))
  (|CallParentFunction DeltaSeconds)
  (bind _asbp_ai_controller_boss (Utilities|Casting|CastToBP_Ai_Controller_Boss (AI|GetAIController self)))
  (Variables|/Game/Ai/Boss/BP_Ai_Controller_Boss.BP_Ai_Controller_Boss_C|SetCurrentHealth _asbp_ai_controller_boss (Variables|/Game/Blueprints/BPC_Player_Stats.BPC_Player_Stats_C|GetCurrent_Health _bpc_player_stats))
  (Variables|/Game/Ai/Boss/BP_Ai_Controller_Boss.BP_Ai_Controller_Boss_C|SetMaxHealth _asbp_ai_controller_boss (Variables|/Game/Blueprints/BPC_Player_Stats.BPC_Player_Stats_C|GetMax_Health _bpc_player_stats)))

(fn ConstructionScript
  (|CallParentFunction))