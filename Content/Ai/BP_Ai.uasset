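; Enemy AI character that fights with a sword and can be stealth-assassinated by the player.
; Behavior-tree attacks run an indexed montage combo, with timer-looped sword sphere traces and a separate single trace damaging "Damageable" actors.
; Damage triggers hit reactions and knockback, then ragdoll and quest elimination on death via BPCPlayerStats.
; Assassination plays a victim montage, delays ragdoll and returns alignment transforms, while camera-facing widgets show health, prompt and investigation icon.
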(event OnComponentBeginOverlap(AssassinationRadius)
  (params (OverlappedComponent :type Primitive%20Component%20Object%20Reference) (OtherActor :type Actor%20Object%20Reference) (OtherComp :type Primitive%20Component%20Object%20Reference) (OtherBodyIndex :type Integer) (bFromSweep :type Boolean) (SweepResult :type Hit%20Result%20Structure%20%28by%20ref%29))
  ;[1 1 1] Assassinate Prompt
  (Utilities|Casting|CastToThirdPersonCharacter OtherActor)
  (Rendering|SetVisibility (Variables|Default|GetAssassinate_Widget) true false))

(event OnComponentEndOverlap(AssassinationRadius)
  (params (OverlappedComponent :type Primitive%20Component%20Object%20Reference) (OtherActor :type Actor%20Object%20Reference) (OtherComp :type Primitive%20Component%20Object%20Reference) (OtherBodyIndex :type Integer))
  ;[1 1 1] Assassinate Prompt
  (Utilities|Casting|CastToThirdPersonCharacter OtherActor)
  (Rendering|SetVisibility (Variables|Default|GetAssassinate_Widget) false false))

(event Custom|Sword_Attack
  ;[1 1 1] Comment
  ;;[1 1 1] Start Attack
  (if (Variables|Default|GetIsAttacking)
    (Variables|Default|SetContinueCombo true)
    (else
      (Variables|Default|SetIsAttacking true)
      (switch int (Variables|Default|GetAttackIndex)
        (:0
          (CallFunction|Attack1))
        (:1
          (CallFunction|Attack2))
        (:2
          (CallFunction|Attack4))))))

(event Custom|Handle_Attack_From_BT
  ;[1 1 1] Comment
  ;;[1 1 1] Attack Input
  (if (Variables|Default|GetCanAttack)
    (CallFunction|SwordAttack)))

(event Custom|Stop_Sword_Trace
  ;[1 1 1] Sword Trace
  (Utilities|Time|ClearandInvalidateTimerbyHandle (Variables|Default|GetSwordTraceLoop)))

(event Custom|Sphere_Trace
  (bind _sphere_trace1 (Variables|Default|GetSphere_Trace1))
  (bind _returnvalue (Transformation|GetWorldLocation _sphere_trace1))
  ;[1 1 1] Sphere Trace (stab/kick attack)
  (bind (_outhit _returnvalue_2) (Collision|SphereTraceByChannel _returnvalue _returnvalue 25.0 "TraceTypeQuery1" false 0 "ForDuration"))
  (if _returnvalue_2
    (if (Actor|ActorHasTag (.HitActor (Collision|BreakHitResult _outhit)) "Damageable")
      (Game|Damage|ApplyDamage (.HitActor (Collision|BreakHitResult _outhit)) 1e+01 0 0)
      (CallFunction|PlaySwordHitSounds)
      (Effects|SpawnEmitteratLocation "/Game/VFX/Particles/Blood/P_Blood_Splat_Cone.P_Blood_Splat_Cone" (.Location (Collision|BreakHitResult _outhit)) (Math|Rotator|MakeRotfromXY (.Normal (Collision|BreakHitResult _outhit)) (.Normal (Collision|BreakHitResult _outhit))) "0.400000,0.400000,0.400000" true "AutoRelease"))))

(event Custom|Play_Sword_Hit_Sounds
  ;[1 1 1] Play sword hit sounds
  (Audio|PlaySoundatLocation "/Game/Audio/Sword_Hits/Sword_Hit_SoundCue.Sword_Hit_SoundCue" (Transformation|GetActorLocation) "0, 0, 0" 1.0 1.0 0.0 "/Game/Audio/SA_Player_Character.SA_Player_Character" 0 0))

(event Custom|Ragdoll
  ;[1 1 1] Ragdoll
  (Utilities|FlowControl|Sequence
    (:then_0
      (Utilities|FlowControl|Delay 2.5)
      (Physics|SetSimulatePhysics (Variables|Character|GetMesh) true))
    (:then_1
      (Utilities|FlowControl|Delay 1.7)
      (Audio|PlaySoundatLocation "/Game/Audio/Grunts_hit/SC_Death.SC_Death" (Transformation|GetActorLocation) "0, 0, 0" 1.0 1.0 0.0 "/Game/Audio/SA_Player_Character.SA_Player_Character" 0 0))))

(event Custom|ToggleInvestigationIcon
  (bind _investigate_widget (Variables|Default|GetInvestigate_Widget))
  (Utilities|FlowControl|FlipFlop
    (:A
      (Rendering|SetVisibility _investigate_widget true false))
    (:B
      (Rendering|SetVisibility _investigate_widget false false))))

(event Custom|Sword_Attack_Combo
  ;[1 1 1] Comment
  ;;[1 1 1] Continue Combo
  (if (Variables|Default|GetContinueCombo)
    (Variables|Default|SetContinueCombo false)
    (switch int (Variables|Default|GetAttackIndex)
      (:0
        (CallFunction|Attack1))
      (:1
        (CallFunction|Attack2))
      (:2
        (CallFunction|Attack4)))
    (else
      (CallFunction|StopAttackCombo))))

(event Custom|Stop_Attack_Combo
  ;[1 1 1] Comment
  ;;[1 1 1] Stop Combo
  (Variables|Default|SetIsAttacking false)
  (Variables|Default|SetAttackIndex 0))

(event Custom|Attack_4
  ;[1 1 1] Comment
  ;;[1 1 1] Attack 4
  (Utilities|FlowControl|DoOnce false :!label _label
    (:Completed
      (Utilities|FlowControl|Delay 0.1)
      (Animation|Montage|PlayMontage (Variables|Character|GetMesh) "/Game/Characters/RPG_Character/Animations/SwordAttacks/Attack3_Montage.Attack3_Montage" (Variables|Default|GetAttackAnimationSpeed)
        (:then
          (Variables|Default|SetAttackIndex 4)
          (goto _label Reset))))))

(event Custom|Attack_1
  ;[1 1 1] Comment
  ;;[1 1 1] Attack 1
  (Utilities|FlowControl|DoOnce false :!label _label
    (:Completed
      (Utilities|FlowControl|Delay 0.1)
      (Animation|Montage|PlayMontage (Variables|Character|GetMesh) "/Game/Characters/RPG_Character/Animations/SwordAttacks/Attack1_Montage.Attack1_Montage" (Variables|Default|GetAttackAnimationSpeed)
        (:then
          (Variables|Default|SetAttackIndex 1)
          (goto _label Reset))))))

(event Custom|Start_Sword_Trace
  ;[1 1 1] Sword Trace
  (bind _returnvalue (Utilities|Time|SetTimerbyEvent (delegate Custom|Sword_Trace_Loop) 0.01 true))
  (Variables|Default|SetSwordTraceLoop _returnvalue))

(event Custom|Attack_2
  ;[1 1 1] Comment
  ;;[1 1 1] Attack 2
  (Utilities|FlowControl|DoOnce false :!label _label
    (:Completed
      (Utilities|FlowControl|Delay 0.1)
      (Animation|Montage|PlayMontage (Variables|Character|GetMesh) "/Game/Characters/RPG_Character/Animations/SwordAttacks/Attack2_Montage.Attack2_Montage" (Variables|Default|GetAttackAnimationSpeed)
        (:then
          (Variables|Default|SetAttackIndex 2)
          (goto _label Reset))))))

(event Custom|Sword_Trace_Loop
  ;[1 1 1] Sword Trace
  (bind (_outhit _returnvalue) (Collision|SphereTraceByChannel (Transformation|GetWorldLocation (Variables|Default|GetSword_Top_Point)) (Transformation|GetWorldLocation (Variables|Default|GetSword_Bottom_Point)) 12.0 "TraceTypeQuery1" false 0 "ForDuration" true "(R=1.000000,G=0.000000,B=0.000000,A=1.000000)" "(R=0.000000,G=1.000000,B=0.000000,A=1.000000)" 0.2))
  (if _returnvalue
    (if (Actor|ActorHasTag (.HitActor (Collision|BreakHitResult _outhit)) "Damageable")
      (Utilities|FlowControl|DoOnce false :!label _label
        (:Completed
          (Game|Damage|ApplyDamage (.HitActor (Collision|BreakHitResult _outhit)) 1e+01 0 0)
          (CallFunction|PlaySwordHitSounds)
          (Effects|SpawnEmitteratLocation "/Game/VFX/Particles/Blood/P_Blood_Splat_Cone.P_Blood_Splat_Cone" (.Location (Collision|BreakHitResult _outhit)) (Math|Rotator|MakeRotfromXY (.Normal (Collision|BreakHitResult _outhit)) (.Normal (Collision|BreakHitResult _outhit))) "0.400000,0.400000,0.400000" true "AutoRelease")
          (Utilities|FlowControl|Delay 0.5)
          (goto _label Reset))))))

(event Custom|Attack_3
  ;[1 1 1] Comment
  ;;[1 1 1] Attack 3 (kick)
  (Utilities|FlowControl|DoOnce false :!label _label
    (:Completed
      (Utilities|FlowControl|Delay 0.1)
      (Animation|Montage|PlayMontage (Variables|Character|GetMesh) "/Game/Characters/RPG_Character/Animations/SwordAttacks/Kick_Montage.Kick_Montage" (Variables|Default|GetAttackAnimationSpeed)
        (:then
          (Variables|Default|SetAttackIndex 3)
          (goto _label Reset))))))

(event EventBeginPlay
  (bind _aswb_dummy_health_bar (Utilities|Casting|CastToWB_Dummy_HealthBar (UserInterface|GetWidget (Variables|Default|GetHealthbar_Widget))))
  (Variables|Default|SetHealth_Bar_UI _aswb_dummy_health_bar))

(event EventTick
  (params (DeltaSeconds :type Float%20%28single-precision%29))
  (Transformation|SetWorldRotation (Variables|Default|GetAssassinate_Widget) (Math|Rotator|FindLookatRotation (Transformation|GetWorldLocation (Variables|Default|GetAssassinate_Widget)) (Transformation|GetWorldLocation (Variables|/Script/Engine.PlayerCameraManager|GetTransformComponent (Game|GetPlayerCameraManager 0)))) false false))

(event Game|Damage|EventAnyDamage
  (params (Damage :type Float%20%28single-precision%29) (DamageType :type Damage%20Type%20Object%20Reference) (InstigatedBy :type Controller%20Object%20Reference) (DamageCauser :type Actor%20Object%20Reference))
  (bind _mesh (Variables|Character|GetMesh))
  ;[1 1 1] Dummy take damage
  (CallFunction|StopAttackCombo)
  (Animation|PlayAnimMontage (Utilities|Array|Get(acopy) (Variables|Default|GetHit_Animations) (Math|Random|RandomIntegerinRange 0 (- (Utilities|Array|Length (Variables|Default|GetHit_Animations)) 1))) 1.0 "None")
  (bind _asthird_person_character (Utilities|Casting|CastToThirdPersonCharacter (Game|GetPlayerCharacter 0)))
  (Character|LaunchCharacter (* (Math|Vector|GetForwardVector (Transformation|GetActorRotation _asthird_person_character)) 7e+02) false false)
  (Audio|PlaySoundatLocation "/Game/Audio/Grunts_hit/death_male_2.death_male_2" (Transformation|GetActorLocation) "0, 0, 0" 1.0 1.0 0.0 "/Game/Audio/SA_Player_Character.SA_Player_Character" 0 0)
  (bind _isplayerdead (Default|DecreaseHealth (Variables|Default|GetBPC_Player_Stats) Damage))
  (if _isplayerdead
    (Collision|SetCollisionObjectType _mesh "ECC_PhysicsBody")
    (Physics|SetSimulatePhysics _mesh true)
    (Audio|PlaySoundatLocation "/Game/Audio/Grunts_hit/SC_Death.SC_Death" (Transformation|GetActorLocation) "0, 0, 0" 1.0 1.0 0.0 "/Game/Audio/SA_Player_Character.SA_Player_Character" 0 0)
    (Rendering|SetVisibility (Variables|Default|GetHealthbar_Widget) false false)
    (Pawn|Components|CharacterMovement|SetMovementMode (Variables|Character|GetCharacterMovement) "MOVE_None" 0)
    (bind _asthird_person_character_2 (Utilities|Casting|CastToThirdPersonCharacter (Game|GetPlayerCharacter 0)))
    (Default|EliminateActor (Variables|/Game/ThirdPersonBP/Blueprints/ThirdPersonCharacter.ThirdPersonCharacter_C|GetBPC_Quest _asthird_person_character_2) self)))

(fn ConstructionScript)

(fn Attack
  (CallFunction|HandleAttackfromBT)
  (return 0.4))

(fn StealthBackAssassin
  (Animation|PlayAnimMontage "/Game/Characters/RPG_Character/Animations/Assassinations/Paired_Knife_Stealth_KidneyAndNeck_Vic_Montage.Paired_Knife_Stealth_KidneyAndNeck_Vic_Montage" 1.0 "None")
  (CallFunction|Ragdoll)
  (Rendering|SetVisibility (Variables|Default|GetAssassinate_Widget) false false)
  (Rendering|SetVisibility (Variables|Default|GetHealthbar_Widget) false false)
  (Pawn|Components|CharacterMovement|SetMovementMode (Variables|Character|GetCharacterMovement) "MOVE_None" 0)
  (return (Transformation|GetWorldLocation (Variables|Default|GetAssassin%20Reference)) (Transformation|GetActorRotation)))