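; A lake water body Blueprint that switches the player's ThirdPersonCharacter in and out of swimming.
; Overlap begin enables Tick and caches the player, then each tick compares the capsule's center height with the lake actor's Z.
; It calls StartSwimming or StopSwimming only when the state flips, with debug spheres and prints.
; When the player leaves the overlap, it disables Tick and stops any active swimming.
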(event Collision|EventActorBeginOverlap
  (params (OtherActor :type Actor%20Object%20Reference))
  (Actor|Tick|SetActorTickEnabled true)
  (if (Actor|ActorHasTag OtherActor "Player")
    (bind _asthird_person_character (Utilities|Casting|CastToThirdPersonCharacter OtherActor))
    (Variables|Default|SetAs%20Third%20Person%20Character _asthird_person_character)
    (Rendering|Debug|DrawDebugSphere (Transformation|GetWorldLocation (Variables|/Script/Engine.Character|GetCapsuleComponent (Variables|Default|GetAs%20Third%20Person%20Character))) 1e+01 12 "(R=0.003206,G=1.000000,B=0.075546,A=1.000000)" 2.0)
    (if (>= (.Z (Math|Vector|BreakVector (Transformation|GetActorLocation))) (.Z (Math|Vector|BreakVector (Transformation|GetWorldLocation (Variables|/Script/Engine.Character|GetCapsuleComponent (Variables|Default|GetAs%20Third%20Person%20Character))))))
      (if (not (Variables|Default|GetisSwimming))
        (Default|StartSwimming _asthird_person_character)
        (Variables|Default|SetisSwimming true)
        (Development|PrintString "swimming"))
      (elif (Variables|Default|GetisSwimming)
        (Default|StopSwimming (Variables|Default|GetAs%20Third%20Person%20Character))
        (Variables|Default|SetisSwimming false)
        (Development|PrintString "stop swimming")))))

(event Collision|EventActorEndOverlap
  (params (OtherActor :type Actor%20Object%20Reference))
  (if (Actor|ActorHasTag OtherActor "Player")
    (Actor|Tick|SetActorTickEnabled false)
    (if (Variables|Default|GetisSwimming)
      (Default|StopSwimming (Variables|Default|GetAs%20Third%20Person%20Character))
      (Variables|Default|SetisSwimming false)
      (Development|PrintString "stop swimming"))))

(event EventTick
  (params (DeltaSeconds :type Float%20%28single-precision%29))
  (bind _as_third_person_character (Variables|Default|GetAs%20Third%20Person%20Character))
  (bind _capsulecomponent (Variables|/Script/Engine.Character|GetCapsuleComponent _as_third_person_character))
  (bind _returnvalue (Transformation|GetWorldLocation _capsulecomponent))
  (Utilities|IsValid (Variables|Default|GetAs%20Third%20Person%20Character)
    (:Is%20Valid
      (Rendering|Debug|DrawDebugSphere _returnvalue 1e+01 12 "(R=0.003206,G=1.000000,B=0.075546,A=1.000000)" 2.0)
      (if (>= (.Z (Math|Vector|BreakVector (Transformation|GetActorLocation))) (.Z (Math|Vector|BreakVector _returnvalue)))
        (if (not (Variables|Default|GetisSwimming))
          (Default|StartSwimming (stale Collision|EventActorBeginOverlap _asthird_person_character))
          (Variables|Default|SetisSwimming true)
          (Development|PrintString "swimming"))
        (elif (Variables|Default|GetisSwimming)
          (Default|StopSwimming (Variables|Default|GetAs%20Third%20Person%20Character))
          (Variables|Default|SetisSwimming false)
          (Development|PrintString "stop swimming"))))))

(fn ConstructionScript)