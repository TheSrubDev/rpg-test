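; Attack component for ThirdPersonCharacter that handles a four-step sword and kick melee combo, plus bow aiming.
; Input during an attack buffers a continue flag, which the combo event uses to play the next montage by AttackIndex or reset.
; A looping timer sphere-traces along the blade, alongside a one-shot trace for stab/kick, damaging "Damageable" actors with blood and sound.
; ShootBow disables attacking and toggles rotation mode and crosshair widget.
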(event Custom|Sword_Attack
  ;[1 1 1] Combo System
  ;;[1 1 1] Start Attack
  (if (Variables|Default|GetIsAttacking)
    (Variables|Default|SetContinueCombo true)
    (else
      (Variables|Default|SetIsAttacking true)
      (switch int (Variables|Default|GetAttackIndex)
        (:0
          (CallFunction|Attack1))
        (:1
          (CallFunction|Attack2))
        (:2
          (CallFunction|Attack3))
        (:3
          (CallFunction|Attack4))))))

(event Custom|Handle_Attack
  ;[1 1 1] Combo System
  ;;[1 1 1] Attack Input
  (if (Variables|Default|GetCanAttack)
    (CallFunction|SwordAttack)))

(event Custom|Stop_Sword_Trace
  ;[1 1 1] Sword Trace
  (Utilities|Time|ClearandInvalidateTimerbyHandle (Variables|Default|GetSwordTraceLoop)))

(event Custom|Sphere_Trace
  (bind _character_bp (Variables|Default|GetCharacter_BP))
  (bind _sphere_trace (Variables|/Game/ThirdPersonBP/Blueprints/ThirdPersonCharacter.ThirdPersonCharacter_C|GetSphere_Trace _character_bp))
  (bind _returnvalue (Transformation|GetWorldLocation _sphere_trace))
  ;[1 1 1] Sphere Trace (stab/kick attack)
  (bind (_outhit _returnvalue_2) (Collision|SphereTraceByChannel _returnvalue _returnvalue 25.0 "TraceTypeQuery1" false 0 "None"))
  (if _returnvalue_2
    (if (Actor|ActorHasTag (.HitActor (Collision|BreakHitResult _outhit)) "Damageable")
      (Game|Damage|ApplyDamage (.HitActor (Collision|BreakHitResult _outhit)) 1e+01 0 0)
      (CallFunction|PlaySwordHitSounds)
      (Effects|SpawnEmitteratLocation "/Game/VFX/Particles/Blood/P_Blood_Splat_Cone.P_Blood_Splat_Cone" (.Location (Collision|BreakHitResult _outhit)) (Math|Rotator|MakeRotfromXY (.Normal (Collision|BreakHitResult _outhit)) (.Normal (Collision|BreakHitResult _outhit))) "0.400000,0.400000,0.400000" true "AutoRelease"))))

(event Custom|Play_Sword_Hit_Sounds
  ;[1 1 1] Play sword hit sounds
  (Audio|PlaySoundatLocation "/Game/Audio/Sword_Hits/Sword_Hit_SoundCue.Sword_Hit_SoundCue" (Transformation|GetActorLocation (Components|GetOwner)) "0, 0, 0" 1.0 1.0 0.0 "/Game/Audio/SA_Player_Character.SA_Player_Character" 0 0))

(event Custom|ShootBow
  (params (IsAimingBow :type Boolean))
  (bind _character_bp (Variables|Default|GetCharacter_BP))
  (bind _character_bp_2 (Variables|Default|GetCharacter_BP))
  (bind _charactermovement (Variables|/Script/Engine.Character|GetCharacterMovement _character_bp))
  (bind _charactermovement_2 (Variables|/Script/Engine.Character|GetCharacterMovement _character_bp_2))
  ;[1 1 1] Shoot bow
  (if (Variables|Default|GetHasBow)
    (Variables|Default|SetCanAttack false)
    (bind _output_get (Variables|Default|SetIsAiming IsAimingBow))
    (if _output_get
      (Default|TakeOutBow _character_bp_2)
      (Variables|/Script/Engine.CharacterMovementComponent|SetbUseControllerDesiredRotation _charactermovement_2 true)
      (Variables|/Script/Engine.CharacterMovementComponent|SetbOrientRotationToMovement _charactermovement_2 false)
      (bind _returnvalue (UserInterface|CreateWidget "/Game/UI/WB_BowCrosshair.WB_BowCrosshair_C"))
      (bind _output_get_2 (Variables|Default|SetBowCrosshairWidget _returnvalue))
      (UserInterface|Viewport|AddtoViewport _output_get_2 0)
      (Development|PrintString "am" (Variables|Default|GetIsAiming))
      (else
        (Default|TakeOutBow _character_bp)
        (Variables|/Script/Engine.CharacterMovementComponent|SetbUseControllerDesiredRotation _charactermovement false)
        (Variables|/Script/Engine.CharacterMovementComponent|SetbOrientRotationToMovement _charactermovement true)
        (Utilities|FlowControl|Delay 0.2)
        (Utilities|IsValid (Variables|Default|GetBowCrosshairWidget)
          (:Is%20Valid
            (Widget|RemovefromParent (Variables|Default|GetBowCrosshairWidget))
            (Variables|Default|SetBowCrosshairWidget 0)))))))

(event Custom|Sword_Attack_Combo
  ;[1 1 1] Combo System
  ;;[1 1 1] Continue Combo
  (if (Variables|Default|GetContinueCombo)
    (Variables|Default|SetContinueCombo false)
    (switch int (Variables|Default|GetAttackIndex)
      (:0
        (CallFunction|Attack1))
      (:1
        (CallFunction|Attack2))
      (:2
        (CallFunction|Attack3))
      (:3
        (CallFunction|Attack4)))
    (else
      (CallFunction|StopAttackCombo))))

(event Custom|Stop_Attack_Combo
  ;[1 1 1] Combo System
  ;;[1 1 1] Stop Combo
  (Variables|Default|SetIsAttacking false)
  (Variables|Default|SetAttackIndex 0))

(event Custom|Attack_4
  ;[1 1 1] Combo System
  ;;[1 1 1] Attack 4
  (Utilities|FlowControl|DoOnce false :!label _label
    (:Completed
      (Utilities|FlowControl|Delay 0.1)
      (Animation|Montage|PlayMontage (Variables|Default|GetCharacter_Mesh) "/Game/Characters/RPG_Character/Animations/SwordAttacks/Attack3_Montage.Attack3_Montage"
        (:then
          (Variables|Default|SetAttackIndex 4)
          (goto _label Reset))))))

(event Custom|Attack_1
  ;[1 1 1] Combo System
  ;;[1 1 1] Attack 1
  (Utilities|FlowControl|DoOnce false :!label _label
    (:Completed
      (Utilities|FlowControl|Delay 0.1)
      (Animation|Montage|PlayMontage (Variables|Default|GetCharacter_Mesh) "/Game/Characters/RPG_Character/Animations/SwordAttacks/Attack1_Montage.Attack1_Montage"
        (:then
          (Variables|Default|SetAttackIndex 1)
          (goto _label Reset))))))

(event Custom|Start_Sword_Trace
  ;[1 1 1] Sword Trace
  (bind _returnvalue (Utilities|Time|SetTimerbyEvent (delegate Custom|Sword_Trace_Loop) 0.01 true))
  (Variables|Default|SetSwordTraceLoop _returnvalue))

(event Custom|Attack_2
  ;[1 1 1] Combo System
  ;;[1 1 1] Attack 2
  (Utilities|FlowControl|DoOnce false :!label _label
    (:Completed
      (Utilities|FlowControl|Delay 0.1)
      (Animation|Montage|PlayMontage (Variables|Default|GetCharacter_Mesh) "/Game/Characters/RPG_Character/Animations/SwordAttacks/Attack2_Montage.Attack2_Montage"
        (:then
          (Variables|Default|SetAttackIndex 2)
          (goto _label Reset))))))

(event Custom|Sword_Trace_Loop
  ;[1 1 1] Sword Trace
  (bind (_outhit _returnvalue) (Collision|SphereTraceByChannel (Transformation|GetWorldLocation (Variables|/Game/ThirdPersonBP/Blueprints/ThirdPersonCharacter.ThirdPersonCharacter_C|GetSword_Top_Point (Variables|Default|GetCharacter_BP))) (Transformation|GetWorldLocation (Variables|/Game/ThirdPersonBP/Blueprints/ThirdPersonCharacter.ThirdPersonCharacter_C|GetSword_Bottom_Point (Variables|Default|GetCharacter_BP))) 12.0 "TraceTypeQuery1" false 0 "None" true "(R=1.000000,G=0.000000,B=0.000000,A=1.000000)" "(R=0.000000,G=1.000000,B=0.000000,A=1.000000)" 0.2))
  (if _returnvalue
    (if (Actor|ActorHasTag (.HitActor (Collision|BreakHitResult _outhit)) "Damageable")
      (Utilities|FlowControl|DoOnce false :!label _label
        (:Completed
          (Game|Damage|ApplyDamage (.HitActor (Collision|BreakHitResult _outhit)) 1e+01 0 0)
          (CallFunction|PlaySwordHitSounds)
          (Effects|SpawnEmitteratLocation "/Game/VFX/Particles/Blood/P_Blood_Splat_Cone.P_Blood_Splat_Cone" (.Location (Collision|BreakHitResult _outhit)) (Math|Rotator|MakeRotfromXY (.Normal (Collision|BreakHitResult _outhit)) (.Normal (Collision|BreakHitResult _outhit))) "0.400000,0.400000,0.400000" true "AutoRelease")
          (Utilities|FlowControl|Delay 0.5)
          (goto _label Reset))))))

(event Custom|Attack_3
  ;[1 1 1] Combo System
  ;;[1 1 1] Attack 3 (kick)
  (Utilities|FlowControl|DoOnce false :!label _label
    (:Completed
      (Utilities|FlowControl|Delay 0.1)
      (Animation|Montage|PlayMontage (Variables|Default|GetCharacter_Mesh) "/Game/Characters/RPG_Character/Animations/SwordAttacks/Kick_Montage.Kick_Montage"
        (:then
          (Variables|Default|SetAttackIndex 3)
          (goto _label Reset))))))

(event EventBeginPlay
  ;[1 1 1] Cast to Character
  (bind _asthird_person_character (Utilities|Casting|CastToThirdPersonCharacter (Components|GetOwner)))
  (Variables|Default|SetCharacter_BP _asthird_person_character)
  (Variables|Default|SetCharacter_Mesh (Variables|/Script/Engine.Character|GetMesh _asthird_person_character)))