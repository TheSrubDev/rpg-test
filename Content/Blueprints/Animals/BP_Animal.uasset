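; BP_Animal is an AI animal pawn that roams, chases the player on sight and attacks in melee.
; It wanders between random reachable points, re-picking only after a successful move, and replays its attack sound at random intervals.
; PawnSensing sightings of Player-tagged pawns trigger a move toward the player, then an attack montage gated by IsAttacking.
; The montage notify runs a forward sphere trace that applies AttackDamage to the pawn hit.
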(event OnSeePawn(PawnSensing)
  (params (Pawn :type Pawn%20Object%20Reference))
  (bind _returnvalue (Transformation|GetActorLocation))
  (if (Actor|ActorHasTag Pawn "Player")
    (AI|AIMoveTo self "0, 0, 0" (Game|GetPlayerCharacter 0) 275.0 false
      (:OnSuccess
        (if (not (Variables|Default|GetIsAttacking))
          (Variables|Default|SetIsAttacking true)
          (Animation|Montage|PlayMontage (Variables|Character|GetMesh) (Variables|Default|GetAttackMontage)
            (:then
              (Audio|PlaySoundatLocation (Variables|Default|GetAnimlaAttackSound) (Transformation|GetActorLocation) "0, 0, 0" 1.0 1.0 0.0 "/Game/Audio/SA_Player_Character.SA_Player_Character" 0 0))
            (:OnCompleted
              (Variables|Default|SetIsAttacking false))
            (:OnNotifyBegin
              (bind (_outhit _returnvalue_2) (Collision|SphereTraceForObjects _returnvalue (+ (* (Math|Vector|GetForwardVector (Transformation|GetActorRotation)) 2.5e+02) _returnvalue) 1.3e+02 (Utilities|Array|MakeArray "ObjectTypeQuery3") false 0 "ForDuration"))
              (if _returnvalue_2
                (Game|Damage|ApplyDamage (.HitActor (Collision|BreakHitResult _outhit)) (Variables|Default|GetAttackDamage) 0 0)))))))))

(event Custom|Animal%20Wandering
  (AI|AIMoveTo self (.RandomLocation (AI|Navigation|GetRandomReachablePointinRadius (Transformation|GetActorLocation) 5e+03 0 0)) 0 5.0 false
    (:OnSuccess
      (Utilities|FlowControl|Delay 3.0)
      (CallFunction|AnimalWandering))))

(event EventBeginPlay
  (CallFunction|AnimalWandering)
  (Utilities|FlowControl|Delay (Math|Random|RandomFloatinRange 7.0 16.0) :!label _label)
  (Audio|PlaySoundatLocation (Variables|Default|GetAnimlaAttackSound) (Transformation|GetActorLocation) "0, 0, 0" 1.0 1.0 0.0 "/Game/Audio/SA_Player_Character.SA_Player_Character" 0 0)
  (goto _label))

(fn ConstructionScript)